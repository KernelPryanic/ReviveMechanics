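; Buff component for an "unconscious issues" effect that steadily raises the afflicted character's Corruption energy.
; On start it caches the owning character's energy receiver component.
; Each buff tick, after the parent logic, it adds a small amount of Corruption through that receiver.
; Once Corruption reaches a high threshold, the next tick jumps it straight to a fixed ceiling rather than continuing gradually.
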(event EventGameplayEffecttoApplyonBuffTick
  (bind _energyreceiverref (Variables|Default|GetEnergyReceiverRef))
  (bind _returnvalue (Class|EnergyReceiverComponent|GetEnergy _energyreceiverref "EnergyType_Corruption"))
  (|CallParentFunction)
  (Utilities|IsValid (Variables|Default|GetEnergyReceiverRef)
    (:Is%20Valid
      (if (< _returnvalue 925.0)
        (Class|EnergyReceiverComponent|ModifyEnergy (Variables|Default|GetEnergyReceiverRef) "EnergyType_Corruption" 0.5)
        (elif (< _returnvalue 1e+03)
          (Class|EnergyReceiverComponent|ModifyEnergy (Variables|Default|GetEnergyReceiverRef) "EnergyType_Corruption" (- 1e+03 _returnvalue)))))))

(event EventStartBuff
  (params (BuffPotency :type Integer) (OwningCharacter :type Conan%20Character%20Object%20Reference) (Instigator :type Controller%20Object%20Reference))
  (|CallParentFunction BuffPotency OwningCharacter Instigator)
  (Variables|Default|SetEnergyReceiverRef (Actor|GetComponentbyClass (Variables|Default|GetOwningCharacter) "/Game/Systems/BPEnergyReceiver.BPEnergyReceiver_C")))