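; Player controller component that plugs the revive mechanic into the game's existing UI: a radial menu entry and an admin settings panel.
; After waiting for a pawn, it hooks GUI module activation signals to add a Revive item when the selected character is unconscious.
; It also injects a button and page into the server settings widget, enabled only for admins, whose controls call setters on the pawn's AC_ReviveMechanics.
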(event Custom|IconToWheel
  (params (module :type GUI%20Module%20Object%20Reference) (isActive :type Boolean))
  ;[1 1 1] Add revive icon to radial menu
  (if isActive
    (bind _windowroot (|GUIModuleActivate module true false false)
      (:OnActivate
        (bind (_radialmenuentry _targetplayercharacter) (CallFunction|AddReviveIcontoRadialMenu _windowroot))
        (EventDispatchers|AssignSignalClicked _radialmenuentry (delegate Custom|Revive))))))

(event Custom|OnTimeChanged
  (params (Value :type Float%20%28single-precision%29))
  (bind _time (CallFunction|ConvertSliderValuetoTime Value))
  (Rendering|Components|TextRender|SetText (Variables|/Game/Mods/ReviveMechanics/Blueprints/UI/WBP_Settings.WBP_Settings_C|GetTB_UnconsciousTime (Variables|Default|GetReviveSettingsWidget)) (Utilities|Text|ToText(Integer) _time))
  (Default|SetTotalTimeServer (Variables|Default|GetReviveMechanics) _time))

(event Custom|Revive
  (params (menuEntry :type Radial%20Menu%20Entry%20Object%20Reference))
  ;[1 1 1] Revive action on radial menu icon
  (Default|Revive (Actor|GetComponentbyClass (Variables|Default|GetControlledPlayerCharacter) "/Game/Mods/ReviveMechanics/Blueprints/AC_ReviveMechanics.AC_ReviveMechanics_C") (stale Custom|IconToWheel _targetplayercharacter)))

(event Custom|OnDeathOnTimerSwitch
  (params (bIsChecked :type Boolean))
  (Default|SetDeathonTimerServer (Variables|Default|GetReviveMechanics) bIsChecked))

(event Custom|OnSuicideDecisionDialogueSwitch
  (params (bIsChecked :type Boolean))
  (Default|SetSuicideDecisionDialogue (Variables|Default|GetReviveMechanics) bIsChecked))

(event Custom|SetupSettings
  (params (module :type GUI%20Module%20Object%20Reference) (isActive :type Boolean))
  (if isActive
    (bind _windowroot (|GUIModuleActivate module true false false)
      (:OnActivate
        (bind _asw_settings (Utilities|Casting|CastToW_Settings _windowroot))
        (Variables|Default|SetServerSettingsWidget (Variables|/Game/UI/MainMenu/Settings/W_Settings.W_Settings_C|GetW_Settings_Server _asw_settings))
        (CallFunction|CreateReviveSettingsButton)
        (CallFunction|CreateReviveSettingsMenu)
        (Utilities|FlowControl|Sequence
          (:then_0
            ;[1 1 1] Settings are accessible only to admin
            (bind _asfun_combat_player_controller (Utilities|Casting|CastToFunCombat_PlayerController (Components|GetOwner)))
            (Widget|SetIsEnabled (Variables|Default|GetReviveSettingsWidget) (Class|ConanPlayerController|IsAdmin _asfun_combat_player_controller)))
          (:then_1
            (EventDispatchers|BindEventtoOnClicked (Variables|/Game/Mods/ReviveMechanics/Blueprints/UI/WBP_SettingsButton.WBP_SettingsButton_C|GetButtonMain (Variables|Default|GetReviveSettingButton)) (delegate Custom|ShowSettings)))
          (:then_2
            (EventDispatchers|AssignOnCheckStateChanged (Variables|/Game/Mods/ReviveMechanics/Blueprints/UI/WBP_Settings.WBP_Settings_C|GetCB_ModEnabled (Variables|Default|GetReviveSettingsWidget)) (delegate Custom|OnModEnabledSwitch)))
          (:then_3
            (EventDispatchers|BindEventtoOnValueChanged (Variables|/Game/Mods/ReviveMechanics/Blueprints/UI/WBP_Settings.WBP_Settings_C|GetS_UnconsciousTime (Variables|Default|GetReviveSettingsWidget)) (delegate Custom|OnTimeChanged)))
          (:then_4
            (EventDispatchers|AssignOnCheckStateChanged (Variables|/Game/Mods/ReviveMechanics/Blueprints/UI/WBP_Settings.WBP_Settings_C|GetCB_DeathOnTimer (Variables|Default|GetReviveSettingsWidget)) (delegate Custom|OnDeathOnTimerSwitch)))
          (:then_5
            (EventDispatchers|BindEventtoOnCheckStateChanged (Variables|/Game/Mods/ReviveMechanics/Blueprints/UI/WBP_Settings.WBP_Settings_C|GetCB_SuicideDecisionDialogue (Variables|Default|GetReviveSettingsWidget)) (delegate Custom|OnSuicideDecisionDialogueSwitch))))))))

(event Custom|OnModEnabledSwitch
  (params (bIsChecked :type Boolean))
  (Default|SetEnabledServer (Variables|Default|GetReviveMechanics) bIsChecked))

(event Custom|ShowSettings
  ;[1 1 1] Show the revive mechanics settings menu
  (Class|WidgetSwitcher|SetActiveWidget (Variables|/Game/UI/MainMenu/Settings/W_Settings_Server.W_Settings_Server_C|GetCategorySwitcher (Variables|Default|GetServerSettingsWidget)) (Variables|Default|GetReviveSettingsWidget)))

(event EventBeginPlay
  (bind _asfun_combat_player_controller (Utilities|Casting|CastToFunCombat_PlayerController (Components|GetOwner)))
  (Utilities|FlowControl|Delay 0.2 :!label _label)
  (Utilities|IsValid (Pawn|GetControlledPawn _asfun_combat_player_controller)
    (:Is%20Valid
      (bind _asbase_player_char (Utilities|Casting|CastToBasePlayerChar (Pawn|GetControlledPawn _asfun_combat_player_controller)))
      (bind _output_get (Variables|Default|SetControlledPlayerCharacter _asbase_player_char))
      (Variables|Default|SetReviveMechanics (Actor|GetComponentbyClass _output_get "/Game/Mods/ReviveMechanics/Blueprints/AC_ReviveMechanics.AC_ReviveMechanics_C"))
      (Utilities|FlowControl|Sequence
        (:then_0
          (bind _returnvalue (Class|GUIModuleController|GetModule (Class|GUIModuleController|GetGUIModuleController) "MainRadialMenu"))
          (EventDispatchers|BindEventtoSignalActivated _returnvalue (delegate Custom|IconToWheel)))
        (:then_1
          (bind _returnvalue_2 (Class|GUIModuleController|GetModule (Class|GUIModuleController|GetGUIModuleController) "Settings"))
          (EventDispatchers|BindEventtoSignalActivated _returnvalue_2 (delegate Custom|SetupSettings)))))
    (:Is%20Not%20Valid
      (goto _label))))

(fn AddReviveIcontoRadialMenu
  (params (RadialMenu :type Window%20Root%20Object%20Reference))
  (bind _asfun_combat_player_controller (Utilities|Casting|CastToFunCombat_PlayerController (Game|GetPlayerController 0))
    (:then
      (bind _asbase_player_char (Utilities|Casting|CastToBasePlayerChar (Utilities|ToObject(Interface) (Variables|/Game/Systems/InteractionManager.InteractionManager_C|GetSelectedObject (Default|GetInteractionManager _asfun_combat_player_controller))))
        (:then
          (LocalVariables|SetTargetPlayerCharacterLocal _asbase_player_char)
          (bind _asw_main_radial_menu (Utilities|Casting|CastToW_MainRadialMenu RadialMenu)
            (:then
              (Utilities|IsValid (Variables|/Game/UI/RadialMenus/W_MainRadialMenu.W_MainRadialMenu_C|GetMenu _asw_main_radial_menu)
                (:Is%20Valid
                  (if (Utilities|Enum|Equal(Enum) (Class|ConanCharacter|GetCharacterState (LocalVariables|GetTargetPlayerCharacterLocal)) "Unconscious")
                    (bind _returnvalue (Class|RadialMenu|AddItem (Variables|/Game/UI/RadialMenus/W_MainRadialMenu.W_MainRadialMenu_C|GetMenu _asw_main_radial_menu) (Utilities|Text|ToText(String) (Class|ConanCharacter|GetCharacterName (LocalVariables|GetTargetPlayerCharacterLocal))) "Revive" "/Game/UI/Textures/EmoteIcons/Categories/icon_emote_category_greet.icon_emote_category_greet" "None" -1)))
                  (return _returnvalue (LocalVariables|GetTargetPlayerCharacterLocal)))))
            (:CastFailed
              (return 0 (LocalVariables|GetTargetPlayerCharacterLocal)))))
        (:CastFailed
          (return 0 0))))
    (:CastFailed
      (return 0 0))))

(fn CreateReviveSettingsButton
  (bind _returnvalue (UserInterface|CreateWidget "/Game/Mods/ReviveMechanics/Blueprints/UI/WBP_SettingsButton.WBP_SettingsButton_C" (Game|GetPlayerController 0)))
  (bind _output_get (Variables|Default|SetReviveSettingButton _returnvalue))
  (UserInterface|Viewport|AddtoViewport _output_get 40)
  (bind _assize_box (Utilities|Casting|CastToSizeBox (Class|PanelWidget|GetChildat (Variables|/Game/UI/MainMenu/Settings/W_Settings_Server.W_Settings_Server_C|GetSideMenu (Variables|Default|GetServerSettingsWidget))))
    (:then
      (bind _asvertical_box (Utilities|Casting|CastToVerticalBox (Class|PanelWidget|GetChildat _assize_box))
        (:then
          (Widget|Panel|AddChild _asvertical_box (Variables|Default|GetReviveSettingButton)))
        (:CastFailed
          (Development|PrintString "Revive Mechanics: Check the W_Settings_server structure" :!label _label))))
    (:CastFailed
      (goto _label))))

(fn CreateReviveSettingsMenu
  (Utilities|FlowControl|Sequence
    (:then_0
      (bind _returnvalue (UserInterface|CreateWidget "/Game/Mods/ReviveMechanics/Blueprints/UI/WBP_Settings.WBP_Settings_C" (Game|GetPlayerController 0)))
      (bind _output_get (Variables|Default|SetReviveSettingsWidget _returnvalue))
      (UserInterface|Viewport|AddtoViewport _output_get 40)
      (Widget|Panel|AddChild (Variables|/Game/UI/MainMenu/Settings/W_Settings_Server.W_Settings_Server_C|GetCategorySwitcher (Variables|Default|GetServerSettingsWidget)) (Variables|Default|GetReviveSettingsWidget)))
    (:then_1
      (Class|CheckBox|SetIsChecked (Variables|/Game/Mods/ReviveMechanics/Blueprints/UI/WBP_Settings.WBP_Settings_C|GetCB_ModEnabled (Variables|Default|GetReviveSettingsWidget)) (Variables|/Game/Mods/ReviveMechanics/Blueprints/AC_ReviveMechanics.AC_ReviveMechanics_C|GetEnabled (Variables|Default|GetReviveMechanics))))
    (:then_2
      (bind _value (CallFunction|ConvertTimetoSliderValue (Variables|/Game/Mods/ReviveMechanics/Blueprints/AC_ReviveMechanics.AC_ReviveMechanics_C|GetTotalTime (Variables|Default|GetReviveMechanics))))
      (Class|Slider|SetValue (Variables|/Game/Mods/ReviveMechanics/Blueprints/UI/WBP_Settings.WBP_Settings_C|GetS_UnconsciousTime (Variables|Default|GetReviveSettingsWidget)) _value)
      (Rendering|Components|TextRender|SetText (Variables|/Game/Mods/ReviveMechanics/Blueprints/UI/WBP_Settings.WBP_Settings_C|GetTB_UnconsciousTime (Variables|Default|GetReviveSettingsWidget)) (Utilities|Text|ToText(Integer) (Variables|/Game/Mods/ReviveMechanics/Blueprints/AC_ReviveMechanics.AC_ReviveMechanics_C|GetTotalTime (Variables|Default|GetReviveMechanics)))))
    (:then_3
      (Class|CheckBox|SetIsChecked (Variables|/Game/Mods/ReviveMechanics/Blueprints/UI/WBP_Settings.WBP_Settings_C|GetCB_DeathOnTimer (Variables|Default|GetReviveSettingsWidget)) (Variables|/Game/Mods/ReviveMechanics/Blueprints/AC_ReviveMechanics.AC_ReviveMechanics_C|GetDeathOnTImer (Variables|Default|GetReviveMechanics))))
    (:then_4
      (Class|CheckBox|SetIsChecked (Variables|/Game/Mods/ReviveMechanics/Blueprints/UI/WBP_Settings.WBP_Settings_C|GetCB_SuicideDecisionDialogue (Variables|Default|GetReviveSettingsWidget)) (Variables|/Game/Mods/ReviveMechanics/Blueprints/AC_ReviveMechanics.AC_ReviveMechanics_C|GetSuicideDecisionDialogue (Variables|Default|GetReviveMechanics))))))

(fn ConvertSliderValuetoTime
  (params (Value :type Float%20%28single-precision%29))
  (return (Math|Float|Round (* Value 3e+02))))

(fn ConvertTimetoSliderValue
  (params (Time :type Integer))
  (return (/ (Math|Conversions|ToFloat(Integer) Time) 3e+02)))