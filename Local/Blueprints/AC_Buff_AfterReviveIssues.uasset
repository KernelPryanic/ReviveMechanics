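; AC_Buff_AfterReviveIssues is a buff component that reduces a character's maximum stamina, named as an after-revive debuff.
; On start it subtracts max stamina divided by StaminaPenaltyDiv through a merged stat modifier, then adds the stored amount back when cleared.
; StartBuff also caches the character's hunger system, but the water-drain logic using it is disconnected and the tick effect is empty.
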(event EventStartBuff
  (params (BuffPotency :type Integer) (OwningCharacter :type Conan%20Character%20Object%20Reference) (Instigator :type Controller%20Object%20Reference))
  (bind _returnvalue (Actor|GetComponentbyClass (Variables|Default|GetOwningCharacter) "/Game/Systems/Hunger/BP_HungerSystem.BP_HungerSystem_C"))
  (|CallParentFunction BuffPotency OwningCharacter Instigator)
  (Utilities|IsValid _returnvalue
    (:Is%20Valid
      (Variables|Default|SetHungerSystem _returnvalue))))

(event EventGameplayEffecttoApplyonBuffStart
  (Variables|Default|SetStaminaPenalty (/ (Class|ConanCharacter|GetStaminaMax (Variables|Default|GetOwningCharacter)) (Variables|Default|GetStaminaPenaltyDiv)))
  (Class|ConanCharacter|AddIntStatModifier (Variables|Default|GetOwningCharacter) "StaminaMax" "Buff" "Add" (* (Variables|Default|GetStaminaPenalty) -1) "Merge"))

(event EventGameplayEffecttoApplyonBuffCleared
  (Class|ConanCharacter|AddIntStatModifier (Variables|Default|GetOwningCharacter) "StaminaMax" "Buff" "Add" (Variables|Default|GetStaminaPenalty) "Merge"))

(event EventGameplayEffecttoApplyonBuffTick)

(fn GetEffectDescription
  (return (Utilities|Text|FormatText "Maximum Stamina reduced in {StaminaMaxReduction}." (Variables|Default|GetStaminaPenaltyDiv))))