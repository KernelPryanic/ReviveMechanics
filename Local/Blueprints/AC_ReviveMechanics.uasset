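; Player character component that adds a knocked-out state with a death countdown and item-based revival by other players.
; A one-second server timer runs down while unconscious, then either kills the player or gets them up with a bandage buff.
; Reviving consumes an item from the reviver's backpack and passes on its buffs.
; Unconscious's RepNotify toggles the countdown widget and calls server events to apply state changes, working around the notify not firing server-side.
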(event Custom|KnockOut
  ;[1 1 1] Knock out
  (CallFunction|KnockOutonServer))

(event Custom|OnReviveServer
  ;[1 1 1] For workaround with not firing replication event on server for "Unconscious" variable
  (CallFunction|OnRevive))

(event Custom|OnKnockOutServer
  ;[1 1 1] For workaround with not firing replication event on server for "Unconscious" variable
  (CallFunction|OnKnockOut))

(event Custom|SetTotalTimeServer
  (params (Value :type Integer))
  ;[1 1 1] Setting parameters on server
  (Utilities|IsAdmin
    (:Admin
      (Variables|Default|SetTotalTime Value))))

(event Custom|CountdownOnServer
  ;[1 1 1] Countdown
  (if (Variables|Default|GetUnconscious)
    (bind _output_get (Variables|Default|SetRemainingTime (- (Variables|Default|GetRemainingTime) 1)))
    (if (<= _output_get 0)
      (if (Variables|Default|GetDeathOnTImer)
        (Default|KillCharacterforSure (Variables|Default|GetOwnerPlayerCharacter) (Variables|KillCharacter|GetHitLocation) (Variables|KillCharacter|GetKillerName) (Variables|KillCharacter|GetKiller))
        (Variables|Default|SetUnconscious false)
        (else
          (CallFunction|GetUp))))))

(event Custom|SetEnabledServer
  (params (Value :type Boolean))
  ;[1 1 1] Setting parameters on server
  (Utilities|IsAdmin
    (:Admin
      (Variables|Default|SetEnabled Value))))

(event Custom|SetDeathOnTimerServer
  (params (Value :type Boolean))
  ;[1 1 1] Setting parameters on server
  (Utilities|IsAdmin
    (:Admin
      (Variables|Default|SetDeathOnTImer Value))))

(event Custom|SetSuicideDecisionDialogue
  (params (Value :type Boolean))
  ;[1 1 1] Setting parameters on server
  (Utilities|IsAdmin
    (:Admin
      (Variables|Default|SetSuicideDecisionDialogue Value))))

(event Custom|GetUp
  ;[1 1 1] Self revive
  (CallFunction|GetUponServer))

(event Custom|DeathCountdownShow
  ;[1 1 1] Coundown widget
  (bind _returnvalue (Class|GUIModuleController|ActivateModule (Class|GUIModuleController|GetGUIModuleController) "DeathCountdown" true false))
  (bind _output_get (Variables|Default|SetDeathTimerWidget _returnvalue))
  (UserInterface|Viewport|AddtoViewport _output_get 0))

(event Custom|DeathCountdownHide
  ;[1 1 1] Coundown widget
  (Widget|RemovefromParent (Variables|Default|GetDeathTimerWidget)))

(event Custom|Revive
  (params (TargetPlayerCharacter :type Base%20Player%20Char%20Object%20Reference))
  ;[1 1 1] Revive
  (CallFunction|ReviveonServer TargetPlayerCharacter))

(event Custom|KnockOutOnServer
  ;[1 1 1] Knock out
  (Variables|Default|SetUnconscious true))

(event Custom|ReviveOnServer
  (params (TargetPlayerCharacter :type Base%20Player%20Char%20Object%20Reference))
  (bind _returnvalue (Actor|GetComponentbyClass TargetPlayerCharacter "AC_ReviveMechanics_C"))
  ;[1 1 1] Revive
  (bind (_revive _revivebuffs) (CallFunction|PreRevive))
  (if _revive
    (Variables|AC_ReviveMechanics_C|SetBuffs _returnvalue _revivebuffs)
    (Variables|AC_ReviveMechanics_C|SetUnconscious _returnvalue false)))

(event Custom|Countdown
  (CallFunction|CountdownonServer))

(event Custom|ApplyBuffs
  (params (Buffs :type Array%20of%2001%20BP%20AC%20Buff%20Master%20Class%20References))
  ;[1 1 1] Buffs application
  (CallFunction|ApplyBuffsonServer Buffs))

(event Custom|SetRemaningTimeServer
  (params (Value :type Integer))
  ;[1 1 1] Setting parameters on server
  (Utilities|IsAdmin
    (:Admin
      (Variables|Default|SetRemainingTime Value))))

(event Custom|ApplyBuffsOnServer
  (params (Buffs :type Array%20of%2001%20BP%20AC%20Buff%20Master%20Class%20References))
  ;[1 1 1] Buffs application
  (for _array_element Buffs
    (Default|AddBuff (Variables|/Game/Characters/BaseBPCombat.BaseBPCombat_C|Get00_BP_AC_BuffSystem (Variables|Default|GetOwnerPlayerCharacter)) _array_element)))

(event Custom|GetUpOnServer
  ;[1 1 1] Self revive
  (Variables|Default|SetBuffs (Utilities|Array|MakeArray "/Game/Systems/Buffs/Heal_OverTime/BP_AC_Buff_Bandage_Basic.BP_AC_Buff_Bandage_Basic_C"))
  (Variables|Default|SetUnconscious false))

(event EventBeginPlay
  (bind _asbase_player_char (Utilities|Casting|CastToBasePlayerChar (Components|GetOwner)))
  (Variables|Default|SetOwnerPlayerCharacter _asbase_player_char)
  (Utilities|HasAuthority
    (:Authority
      (Variables|Default|SetRemainingTime (Variables|Default|GetTotalTime))
      (Utilities|Time|SetTimerbyEvent (delegate Custom|Countdown) 1.0 true))))

(fn OnKnockOut
  (bind _ownerplayercharacter (Variables|Default|GetOwnerPlayerCharacter))
  (Utilities|FlowControl|Sequence
    (:then_0
      (Pawn|Components|CharacterMovement|DisableMovement (Variables|/Script/Engine.Character|GetCharacterMovement (Variables|Default|GetOwnerPlayerCharacter)))
      (Variables|/Script/Engine.Actor|SetbCanBeDamaged (Variables|Default|GetOwnerPlayerCharacter) false)
      (Variables|/Script/ConanSandbox.ConanCharacter|SetSenseDetection (Variables|Default|GetOwnerPlayerCharacter) true)
      (Collision|SetCollisionProfileName (Variables|/Script/Engine.Character|GetMesh (Variables|Default|GetOwnerPlayerCharacter)) "Ragdoll" :!class /Script/Engine.PrimitiveComponent)
      (Class|ConanCharacter|SetIntStat _ownerplayercharacter "ConsciousnessCurrent")
      (Class|ConanCharacter|AdjustHealth (Variables|Default|GetOwnerPlayerCharacter) (* (Class|ConanCharacter|GetIntStat _ownerplayercharacter "HealthCurrent" "Full") -1))
      (Class|ConanCharacter|SetCharacterState (Variables|Default|GetOwnerPlayerCharacter) "Unconscious" true))
    (:then_1
      (bind _buff (Default|AddBuff (Variables|/Game/Characters/BaseBPCombat.BaseBPCombat_C|Get00_BP_AC_BuffSystem (Variables|Default|GetOwnerPlayerCharacter)) "/Game/Mods/ReviveMechanics/Blueprints/AC_Buff_unconsciousIssues.AC_Buff_UnconsciousIssues_C" 1 (CallFunction|GetControllerfromActor (Variables|Default|GetOwnerPlayerCharacter))))
      (bind _output_get (Variables|Default|SetActiveDebuff _buff))
      (Variables|/Game/Systems/Buffs/01_BP_AC_Buff_Master.01_BP_AC_Buff_Master_C|SetBuffTicks _output_get 600)
      (Default|ResetBuffTicks (Variables|Default|GetActiveDebuff)))))

(fn OnRevive
  (bind _ownerplayercharacter (Variables|Default|GetOwnerPlayerCharacter))
  (Utilities|FlowControl|Sequence
    (:then_0
      (Variables|/Script/Engine.Actor|SetbCanBeDamaged (Variables|Default|GetOwnerPlayerCharacter) true)
      (Variables|/Script/ConanSandbox.ConanCharacter|SetSenseDetection _ownerplayercharacter false)
      (Class|ConanCharacter|SetIntStat (Variables|Default|GetOwnerPlayerCharacter) "ConsciousnessCurrent" (Variables|/Game/Characters/BaseBPCombat.BaseBPCombat_C|GetDefaultConsciousness _ownerplayercharacter))
      (Class|ConanCharacter|SetCharacterState (Variables|Default|GetOwnerPlayerCharacter) "Passive" true)
      (Collision|SetCollisionProfileName (Variables|/Script/Engine.Character|GetMesh (Variables|Default|GetOwnerPlayerCharacter)) "ConanCharacterMesh" :!class /Script/Engine.PrimitiveComponent)
      (Variables|/Game/Characters/BasePlayerChar.BasePlayerChar_C|SetBreathingMeterValue (Variables|Default|GetOwnerPlayerCharacter) (Variables|/Game/Characters/BasePlayerChar.BasePlayerChar_C|GetBreathingMeterMax (Variables|Default|GetOwnerPlayerCharacter)))
      (Class|CharacterMovementComponent|SetDefaultMovementMode (Variables|/Script/Engine.Character|GetCharacterMovement (Variables|Default|GetOwnerPlayerCharacter))))
    (:then_1
      (Default|ClearBuff (Variables|Default|GetActiveDebuff))
      (Default|AddBuff (Variables|/Game/Characters/BaseBPCombat.BaseBPCombat_C|Get00_BP_AC_BuffSystem (Variables|Default|GetOwnerPlayerCharacter)) "/Game/Mods/ReviveMechanics/Blueprints/AC_Buff_AfterReviveIssues.AC_Buff_AfterReviveIssues_C")
      (Variables|Default|SetRemainingTime (Variables|Default|GetTotalTime)))))

(fn PreRevive
  (bind _ownerplayercharacter (Variables|Default|GetOwnerPlayerCharacter))
  (bind _backpackinventory (Variables|/Game/Characters/BasePlayerChar.BasePlayerChar_C|GetBackpackInventory _ownerplayercharacter))
  (if (Utilities|Enum|NotEqual(Enum) (Class|ConanCharacter|GetCharacterState (Variables|Default|GetOwnerPlayerCharacter)) "Unconscious")
    (for _array_element (Variables|Default|GetReviveItems)
      (LocalVariables|SetTemplateId _array_element)
      (if (Class|ItemInventory|HasItembyTemplateID (Variables|/Game/Characters/BasePlayerChar.BasePlayerChar_C|GetBackpackInventory (Variables|Default|GetOwnerPlayerCharacter)) _array_element 1)
        (bind _asbpgame_item_food (Utilities|Casting|CastToBPGameItemFood (Class|ItemInventory|GetItembyTemplateID (Variables|/Game/Characters/BasePlayerChar.BasePlayerChar_C|GetBackpackInventory (Variables|Default|GetOwnerPlayerCharacter)) (LocalVariables|GetTemplateId))))
        (LocalVariables|SetBuffsLocal (Variables|/Game/Items/Hunger/BPGameItemFood.BPGameItemFood_C|GetBuffs%20On%20Use _asbpgame_item_food))
        (Class|ItemInventory|DeleteItems _backpackinventory (Class|ItemInventory|FindItembyTemplateID _backpackinventory (LocalVariables|GetTemplateId)) 1)
        (return true (LocalVariables|GetBuffsLocal))))
    (return false (LocalVariables|GetBuffsLocal))
    (else
      (return false (LocalVariables|GetBuffsLocal)))))

(fn OnRepUnconscious
  (Utilities|FlowControl|Sequence
    (:then_0
      (Utilities|LocalPlayer
        (:Local
          (if (Variables|Default|GetUnconscious)
            (CallFunction|DeathCountdownShow)
            (else
              (CallFunction|DeathCountdownHide))))))
    (:then_1
      ;[1 1 1] Executes server function only on the owning client. Workaround for not firing rep event for "Unconscious" variable
      (if (Variables|Default|GetUnconscious)
        (CallFunction|OnKnockOutServer)
        (else
          (CallFunction|OnReviveServer))))))

(fn OnRepBuffs
  (CallFunction|ApplyBuffs (Variables|Default|GetBuffs)))

(fn OnRepTotalTime
  (CallFunction|SetRemaningTimeServer (Variables|Default|GetTotalTime)))